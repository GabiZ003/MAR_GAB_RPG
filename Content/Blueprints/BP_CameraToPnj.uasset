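; BP_CameraToPnj is an actor, named as a camera, that frames an NPC (MyPnj) from the player's position.
; On BeginPlay it caches the player pawn as a BP_TopDownCharacter.
; The GoToPlayer event snaps the actor to the player's Scene component and rotates it to look at the MyPnj Scene component.
; Nothing in this file assigns MyPnj or calls GoToPlayer.
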(event `self.ReceiveBeginPlay`
  (`parent.ReceiveBeginPlay`)
  (bind _asbp_top_down_character (cast `/Game/TopDown/Blueprints/BP_TopDownCharacter` (`GameplayStatics.GetPlayerPawn` 0)))
  (set `self.Player` _asbp_top_down_character))

(event `GoToPlayer`
  (bind _returnvalue (`SceneComponent.K2_GetComponentLocation` (`/Game/TopDown/Blueprints/BP_TopDownCharacter.Scene` (`self.Player`))))
  (`self.K2_SetActorTransform` (`KismetMathLibrary.MakeTransform` _returnvalue (`KismetMathLibrary.FindLookAtRotation` _returnvalue (`SceneComponent.K2_GetComponentLocation` (`/Game/Blueprints/Interractable/BP_PNJ.Scene` (`self.MyPnj`)))))))

(fn `UserConstructionScript`)