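; BP_Fire_Child is a fire actor that sets an enemy burning when it attacks, extending a parent Blueprint.
; BeginPlay runs the parent logic, then shows the Niagara effect.
; The Attack event hides that effect and the SMFire component, reveals the IsBurning component on MyEnnemy and calls its Burning function.
; MyEnnemy is not assigned in these graphs.
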(event `self.ReceiveBeginPlay`
  (`parent.ReceiveBeginPlay`)
  (`SceneComponent.SetVisibility` (`self.Niagara`) true false))

(event `self.Attack`
  (bind _myennemy (`self.MyEnnemy`))
  (`SceneComponent.SetVisibility` (`self.Niagara`) false false)
  (`SceneComponent.SetVisibility` (`self.SM_Fire`) false false)
  (`SceneComponent.SetVisibility` (`/Game/TopDown/Blueprints/BP_TopDownCharacterEnemy.IsBurning` _myennemy) true false)
  (`/Game/TopDown/Blueprints/BP_TopDownCharacterEnemy.Burning` _myennemy))

(fn `UserConstructionScript`
  (`parent.UserConstructionScript`))