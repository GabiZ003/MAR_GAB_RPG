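; BP_Bullet is a bullet actor driven by a ProjectileMovement component, with all its setup in BeginPlay.
; It casts the player pawn to BP_TopDownCharacter, then rotates itself to look from its location toward that character's forward vector, used as a target point rather than a direction.
; It then sets the projectile's initial and max speeds, disables gravity and makes rotation follow velocity.
; It contains no overlap or hit logic.
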(event `self.ReceiveBeginPlay`
  (bind _projectilemovement (`self.ProjectileMovement`))
  (bind _asbp_top_down_character (cast `/Game/TopDown/Blueprints/BP_TopDownCharacter` (`GameplayStatics.GetPlayerPawn` 0)))
  (bind _output_get (set `self.Player` _asbp_top_down_character))
  (`self.K2_SetActorRotation` (`KismetMathLibrary.FindLookAtRotation` (`self.K2_GetActorLocation`) (`self.GetActorForwardVector` _output_get)))
  (set `ProjectileMovementComponent.InitialSpeed` 500.0 _projectilemovement)
  (set `ProjectileMovementComponent.MaxSpeed` 1000.0 _projectilemovement)
  (set `ProjectileMovementComponent.ProjectileGravityScale` 0.0 _projectilemovement)
  (set `ProjectileMovementComponent.bRotationFollowsVelocity` true _projectilemovement))

(fn `UserConstructionScript`)