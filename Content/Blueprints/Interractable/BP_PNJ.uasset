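; BP_PNJ is an interactable NPC that switches the game to a conversation-style camera view.
; A FlipFlop on Interract toggles the text, player movement and a view blend between the NPC's camera and the player's pawn.
; The NPC camera copies the transform of a lazily spawned, reused BP_CameraToPnj helper.
; After a delay, a Timeline lerps the NPC's yaw from its initial rotation toward the player.
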(event `self.ReceiveBeginPlay`
  (bind (_returnvalue_roll _returnvalue_pitch _returnvalue_yaw) (`KismetMathLibrary.BreakRotator` (`SceneComponent.K2_GetComponentRotation` (`self.DefaultSceneRoot`))))
  (`parent.ReceiveBeginPlay`)
  (set `self.MyBodyRotation` _returnvalue_yaw)
  (`KismetSystemLibrary.PrintString` (`KismetStringLibrary.Conv_DoubleToString` (`self.MyBodyRotation`))))

(event `self.Interract`
  (bind _playercontroller (`/Game/Blueprints/BP_FL_Shortcut.GetTopDownController`))
  (bind _playercontroller_2 (`/Game/Blueprints/BP_FL_Shortcut.GetTopDownController`))
  (bind _returnvalue (`SceneComponent.K2_GetComponentLocation` (`/Game/TopDown/Blueprints/BP_TopDownCharacter.Scene` (`self.Player`))))
  (`/Engine/EditorBlueprintResources/StandardMacros.FlipFlop`
    (:`A`
      (`self.CameraGoTo`
        (:`then`
          _)
        (:`else`
          (bind _returnvalue_2 (`|SpawnActorFromClass` "/Game/Blueprints/BP_CameraToPnj.BP_CameraToPnj_C" (`KismetMathLibrary.MakeTransform` _returnvalue (`KismetMathLibrary.FindLookAtRotation` _returnvalue (`SceneComponent.K2_GetComponentLocation` (`self.Scene`)))) "Undefined" "MultiplyWithRoot" null null))
          (set `self.CameraGoTo` _returnvalue_2)
          (set `/Game/Blueprints/BP_CameraToPnj.MyPnj` self (`self.CameraGoTo`))))
      (`/Game/Blueprints/BP_CameraToPnj.GoToPlayer` (`self.CameraGoTo`))
      (`self.MyCameraToPlayer`)
      (`SceneComponent.SetVisibility` (`self.TextRender1`) true false)
      (`PlayerController.SetViewTargetWithBlend` _playercontroller_2 self 1.0 "VTBlend_Linear" 1.0 false)
      (set `/Game/TopDown/Blueprints/BP_TopDownController.ShouldMove` false _playercontroller_2)
      (`KismetSystemLibrary.Delay` 1.0)
      (`TimelineComponent.PlayFromStart` (`self.Timeline`)))
    (:`B`
      (`SceneComponent.SetVisibility` (`self.TextRender1`) false false)
      (`PlayerController.SetViewTargetWithBlend` _playercontroller (`Controller.K2_GetPawn` _playercontroller) 1.0 "VTBlend_Linear" 0.0 false)
      (set `/Game/TopDown/Blueprints/BP_TopDownController.ShouldMove` true _playercontroller))))

(event `MyCameraToPlayer`
  (`SceneComponent.K2_SetWorldTransform` (`self.Camera`) (`self.GetTransform` (`self.CameraGoTo`)) false false))

(fn `UserConstructionScript`)